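; Game mode for a two-player Arkanoid game that builds the level, assigns spawn points and handles the restart.
; BeginPlay spawns BP_Level at the world origin.
; ReadyPlayer collects controllers and, once two are stored, returns both to game-only input and restarts the game.
; The ChoosePlayerStart override claims the first free PlayerStart by tagging it "Taken", so players get separate starts.
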(event `self.ReceiveBeginPlay`
  (`|SpawnActorFromClass` "/Game/ArkonoidGame/Blueprints/BP_Level.BP_Level_C" (`KismetMathLibrary.MakeTransform` (0.0 0.0 0.0)) "Undefined" "OverrideRootScale" null null))

(event `ReadyPlayer`
  (params (PlayerController :type "PlayerController Object Reference"))
  (bind _playerscontrollers (`self.PlayersControllers`))
  ;[1 1 1] Проверяет все ли игроки нажали продолжить
  (`KismetArrayLibrary.Array_Add` _playerscontrollers PlayerController)
  (if (== (`KismetArrayLibrary.Array_Length` _playerscontrollers) 2)
    (for _array_element (`self.PlayersControllers`)
      (`WidgetBlueprintLibrary.SetInputMode_GameOnly` _array_element))
    (`self.RestartGame`)))

(fn `ChoosePlayerStart`
  (params (Player :type "Controller Object Reference"))
  (returns (ReturnValue :type "Actor Object Reference"))
  (bind _outactors (`GameplayStatics.GetAllActorsOfClass` "/Script/Engine.PlayerStart"))
  (for _array_element _outactors
    (if (!= (`PlayerStart.PlayerStartTag` _array_element) "Taken")
      (`|ExecutionSequence`
        (:`then_0`
          (break))
        (:`then_1`
          (set `PlayerStart.PlayerStartTag` "Taken" _array_element)
          (return _array_element))))))

(fn `UserConstructionScript`)