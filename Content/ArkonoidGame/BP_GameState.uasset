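; Game state Blueprint for an Arkanoid game that tracks bricks, balls and lives and decides win or loss.
; Registered bricks and balls remove themselves through OnDestroyed bindings: clearing all bricks wins, while losing the last ball costs a life, and zero lives loses.
; Win, lose and life changes broadcast through dispatchers, and either ending freezes remaining balls.
; Make2Ball duplicates every ball, staging spawns in a temporary array before registering them.
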(event `AddBrick`
  (params (NewItem :type "/Game/ArkonoidGame/Blueprints/BP_Brick Object Reference (by ref)"))
  ;[1 1 1] Добавляет кирпичь в массив и при его уничтожении проверяет, уничтожены ли все кирпичи
  (`KismetArrayLibrary.Array_Add` (`self.Bricks`) NewItem)
  (add `self.OnDestroyed` NewItem (delegate `OnDestroyed_Event`)))

(event `OnDestroyed_Event` :!signature `self.OnDestroyed`
  (params (DestroyedActor :type "Actor Object Reference"))
  (bind _bricks (`self.Bricks`))
  ;[1 1 1] Добавляет кирпичь в массив и при его уничтожении проверяет, уничтожены ли все кирпичи
  (`KismetArrayLibrary.Array_RemoveItem` _bricks (cast `/Game/ArkonoidGame/Blueprints/BP_Brick` DestroyedActor :!pure true))
  (if (`KismetArrayLibrary.Array_IsEmpty` _bricks)
    (`self.OnWinEvent`)
    (`self.StopAllBalls`)))

(event `Addball`
  (params (NewItem :type "/Game/ArkonoidGame/Blueprints/BP_Ball Object Reference (by ref)"))
  ;[1 1 1] Добавялет в мяч в массив и при унижчтожении мяча проверяет был ли это последний мяч и сотвественно делает проигрыш или отнимает жизнь
  (`KismetArrayLibrary.Array_Add` (`self.Balls`) NewItem)
  (add `self.OnDestroyed` NewItem (delegate `OnDestroyed_Event_0`)))

(event `OnDestroyed_Event_0` :!signature `self.OnDestroyed`
  (params (DestroyedActor :type "Actor Object Reference"))
  (bind _balls (`self.Balls`))
  ;[1 1 1] Добавялет в мяч в массив и при унижчтожении мяча проверяет был ли это последний мяч и сотвественно делает проигрыш или отнимает жизнь
  (`KismetArrayLibrary.Array_RemoveItem` _balls (cast `/Game/ArkonoidGame/Blueprints/BP_Ball` DestroyedActor :!pure true))
  (if (`KismetArrayLibrary.Array_IsEmpty` _balls)
    (bind _result (`/Engine/EditorBlueprintResources/StandardMacros.DecrementInt` (`self.Lifes`))
      (:`  `
        (`self.OnLifesChangedEvent` _result)
        (if (== _result 0)
          (`self.OnLoseEvent`)
          (`self.StopAllBalls`))))))

(event `OnLoseEvent`
  (`self.OnLose`))

(event `OnWinEvent`
  (`self.OnWin`))

(event `OnLifesChangedEvent`
  (params (Lifes :type Integer))
  (`self.OnLifesChanged` Lifes))

(event `AddLife`
  ;[1 1 1] Добавляет жизнь
  (bind _result (`/Engine/EditorBlueprintResources/StandardMacros.IncrementInt` (`self.Lifes`))
    (:`  `
      (`self.OnLifesChanged` _result))))

(event `Make2Ball`
  ;[1 1 1] Удваивает каждый шар
  (for _array_element (`self.Balls`)
    (`/Engine/EditorBlueprintResources/StandardMacros.IsValid` _array_element
      (:`Is Valid`
        (bind _returnvalue (`|SpawnActorFromClass` "/Game/ArkonoidGame/Blueprints/BP_Ball.BP_Ball_C" (`self.GetTransform` _array_element) "AlwaysSpawn" "OverrideRootScale" null true null))
        (`KismetArrayLibrary.Array_Add` (`self.TempArr`) _returnvalue))))
  (for _array_element_2 (`self.TempArr`)
    (`self.Addball` _array_element_2))
  (`KismetArrayLibrary.Array_Clear` (`self.TempArr`)))

(fn `StopAllBalls`
  (for _array_element (`self.Balls`)
    (set `/Game/ArkonoidGame/Blueprints/BP_Ball.CanMove` false _array_element)))

(fn `UserConstructionScript`)