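; BP_Ball is the ball actor for an Arkanoid-style game, which moves on the XY plane and bounces off whatever blocks it.
; After a short delay from BeginPlay, it enables movement with a fixed X heading and random Y component.
; Tick calls MulticastMovement, intended as server-driven movement, which applies a swept offset from direction, speed and delta time.
; Blocking hits reflect the direction about the surface normal, without physics simulation.
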(event `self.ReceiveBeginPlay`
  (`self.Delay and rand dir`))

(event `Delay and rand dir`
  (`KismetSystemLibrary.Delay` 3.0)
  (set `self.CanMove` true)
  (set `self.Direction` (`KismetMathLibrary.MakeVector` -1.0 (`KismetMathLibrary.RandomFloatInRange` -1.0 1.0))))

(event `self.ReceiveTick`
  (params (DeltaSeconds :type "Float (single-precision)"))
  ;[1 1 1] Передвижение на сервере
  (if (`self.CanMove`)
    (`self.MulticastMovement` DeltaSeconds)))

(event `MulticastMovement`
  (params (NewParam :type "Float (double-precision)"))
  (bind (_returnvalue_x _returnvalue_y) (`KismetMathLibrary.BreakVector` (* (`self.Direction`) (* NewParam (`self.Speed`)))))
  ;[1 1 1] Передвижение на сервере
  (bind _sweephitresult (`self.K2_AddActorWorldOffset` (`KismetMathLibrary.MakeVector` _returnvalue_x _returnvalue_y) true))
  (bind (_bblockinghit _binitialoverlap _time _distance _location _impactpoint _normal) (`GameplayStatics.BreakHitResult` _sweephitresult))
  ;;[1 1 1] Отскок
  (if _bblockinghit
    (set `self.Direction` (`KismetMathLibrary.GetReflectionVector` (`self.Direction`) _normal))))

(fn `UserConstructionScript`)