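; BP_Platform is the player's paddle in an Arkanoid-style game, moving sideways and collecting bonuses.
; MoveRight axis input passes through a chain of custom events, commented as server-side movement, to a swept local X offset scaled by PlatformSpeed.
; Overlapping a BP_Bonus calls AddLife or Make2Ball on BP_GameState according to the bonus type, then destroys the bonus.
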(event `InputAxis|MoveRight`
  (params (AxisValue :type "Float (single-precision)"))
  ;[1 1 1] Передвижение платформы на сервере
  (`self.MovePlatform` AxisValue))

(event `MovePlatform`
  (params (Value :type "Float (double-precision)"))
  ;[1 1 1] Передвижение платформы на сервере
  (`self.MovePlatformAll` Value))

(event `MovePlatformAll`
  (params (Axis :type "Float (double-precision)"))
  ;[1 1 1] Передвижение платформы на сервере
  (`SceneComponent.K2_AddLocalOffset` (`self.Platform`) (`KismetMathLibrary.MakeVector` (* Axis (`self.PlatformSpeed`))) true false))

(event `self.ReceiveActorBeginOverlap`
  (params (OtherActor :type "Actor Object Reference"))
  ;[1 1 1] Если с платформой столкнулся бонус, то он применяется
  (`self.ApplyBonus` OtherActor))

(event `ApplyBonus`
  (params (NewParam :type "Actor Object Reference"))
  (bind _asbp_game_state (cast `/Game/ArkonoidGame/BP_GameState` (`GameplayStatics.GetGameState`) :!pure true))
  ;[1 1 1] Если с платформой столкнулся бонус, то он применяется
  (bind _asbp_bonus (cast `/Game/ArkonoidGame/Blueprints/BP_Bonus` NewParam))
  (if (`|EnumEquality` (`/Game/ArkonoidGame/Blueprints/BP_Bonus.Type` _asbp_bonus) "NewEnumerator0")
    (`/Game/ArkonoidGame/BP_GameState.AddLife` _asbp_game_state)
    (else
      (`/Game/ArkonoidGame/BP_GameState.Make2Ball` _asbp_game_state)))
  (`self.K2_DestroyActor` _asbp_bonus))

(fn `UserConstructionScript`)