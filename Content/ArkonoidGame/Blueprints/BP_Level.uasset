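; Level actor for an Arkanoid-style game that builds a random arena and handles balls leaving it.
; On BeginPlay, a server event spawns bricks at 50% chance per cell of a random-sized grid, adds the first ball, and fits walls and ceiling to the grid.
; Bricks and balls register with BP_GameState.
; A trigger box destroys escaped balls through a server event, spawning a replacement if lives remain and no balls are left.
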(event `self.ReceiveBeginPlay`
  ;[1 1 1] Спавн левела на сервере
  (`self.ServerSpawn`))

(event `ServerSpawn`
  ;[1 1 1] Спавн левела на сервере
  (`self.GenerateLevel`))

(event `self.Box.OnComponentBeginOverlap`
  (params (OverlappedComponent :type "PrimitiveComponent Object Reference") (OtherActor :type "Actor Object Reference") (OtherComp :type "PrimitiveComponent Object Reference") (OtherBodyIndex :type Integer) (bFromSweep :type Boolean) (SweepResult :type "HitResult Structure (by ref)"))
  ;[1 1 1] При поподании мяча за уровень, проверяется если ли жизни и был ли этот мяч единственный, если условие верно, то спавнится новый мяч
  (`self.Server_BallOutArena` OtherActor))

(event `Server_BallOutArena`
  (params (Actor :type "Actor Object Reference"))
  (bind _asbp_game_state (cast `/Game/ArkonoidGame/BP_GameState` (`GameplayStatics.GetGameState`) :!pure true))
  ;[1 1 1] При поподании мяча за уровень, проверяется если ли жизни и был ли этот мяч единственный, если условие верно, то спавнится новый мяч
  (bind _asbp_ball (cast `/Game/ArkonoidGame/Blueprints/BP_Ball` Actor))
  (`self.K2_DestroyActor` _asbp_ball)
  (if (and (> (`/Game/ArkonoidGame/BP_GameState.Lifes` _asbp_game_state) 0) (`KismetArrayLibrary.Array_IsEmpty` (`/Game/ArkonoidGame/BP_GameState.Balls` _asbp_game_state)))
    (bind _returnvalue (`|SpawnActorFromClass` "/Game/ArkonoidGame/Blueprints/BP_Ball.BP_Ball_C" (`SceneComponent.K2_GetComponentToWorld` (`self.BollSpawnPoint`)) "Undefined" "OverrideRootScale" null false null))
    (`/Game/ArkonoidGame/BP_GameState.Addball` _asbp_game_state _returnvalue)))

(fn `GenerateLevel`
  (locals (I :type Integer) (J :type Integer))
  (`self.RandomRowsAndColomns`)
  ;[1 1 1] Спавн кирпичей
  (for _index (range (`self.Colomns`))
    (bind _output_get (set `local.I` _index))
    (for _index_2 (range (`self.Rows`))
      (bind _output_get_2 (set `local.J` _index_2))
      ;;[1 1 1] 50% шанс, что кирпич заспавнится
      (if (`KismetMathLibrary.RandomBool`)
        (bind _brick (`self.SpawnBrick` _output_get _output_get_2))
        (bind _asbp_game_state (cast `/Game/ArkonoidGame/BP_GameState` (`GameplayStatics.GetGameState`)))
        (`/Game/ArkonoidGame/BP_GameState.AddBrick` _asbp_game_state _brick))))
  ;[1 1 1] Спавн начального мяча
  (bind _returnvalue (`|SpawnActorFromClass` "/Game/ArkonoidGame/Blueprints/BP_Ball.BP_Ball_C" (`SceneComponent.K2_GetComponentToWorld` (`self.BollSpawnPoint`)) "Undefined" "OverrideRootScale" null false null))
  (bind _asbp_game_state_2 (cast `/Game/ArkonoidGame/BP_GameState` (`GameplayStatics.GetGameState`)))
  (`/Game/ArkonoidGame/BP_GameState.Addball` _asbp_game_state_2 _returnvalue)
  (`self.GerateWallsAndUpFloor`))

(fn `GerateWallsAndUpFloor`
  (`SceneComponent.K2_SetWorldTransform` (`self.LeftWall`) (`KismetMathLibrary.MakeTransform` (`KismetMathLibrary.MakeVector` (`KismetMathLibrary.Conv_IntToDouble` (/ (* (+ 2 2 (- (`self.Rows`) 1)) 50) -2)) (`KismetMathLibrary.Conv_IntToDouble` (+ (/ (+ (* (`self.Colomns`) 100) (* (- (`self.Colomns`) 1) 50)) 2) 50))) (struct :`Yaw` 90.0 :`Roll` -90.0) (`KismetMathLibrary.MakeVector` 0.1 1.0 (+ (* (`self.Rows`) 0.375) 2.5 0.0))) false false)
  (`SceneComponent.K2_SetWorldTransform` (`self.RightWall`) (`KismetMathLibrary.MakeTransform` (`KismetMathLibrary.MakeVector` (`KismetMathLibrary.Conv_IntToDouble` (/ (* (+ 2 2 (- (`self.Rows`) 1)) 50) -2)) (`KismetMathLibrary.Conv_IntToDouble` (* (+ (/ (+ (* (`self.Colomns`) 100) (* (- (`self.Colomns`) 1) 50)) 2) 50) -1))) (struct :`Yaw` 90.0 :`Roll` -90.0) (`KismetMathLibrary.MakeVector` 0.1 1.0 (+ (* (`self.Rows`) 0.375) 2.5 0.0))) false false)
  (`SceneComponent.K2_SetWorldTransform` (`self.UpFloor`) (`KismetMathLibrary.MakeTransform` (`KismetMathLibrary.MakeVector` (* (+ (* (`self.Rows`) 37.5) 250.0) -1.0)) (struct :`Yaw` 90.0 :`Roll` -90.0) (`KismetMathLibrary.MakeVector` (+ (* 1.5 (`self.Colomns`)) 0.5) 1.0 0.1)) false false))

(fn `RandomRowsAndColomns`
  (set `self.Rows` (`KismetMathLibrary.RandomIntegerInRange` 4 8))
  (set `self.Colomns` (`KismetMathLibrary.RandomIntegerInRange` 4 8)))

(fn `SpawnBrick`
  (params (I :type Integer) (J :type Integer))
  (returns (Brick :type "/Game/ArkonoidGame/Blueprints/BP_Brick Object Reference"))
  (bind _returnvalue (`|SpawnActorFromClass` "/Game/ArkonoidGame/Blueprints/BP_Brick.BP_Brick_C" (`KismetMathLibrary.MakeTransform` (`KismetMathLibrary.MakeVector` (+ (* (`local.J`) -37.5) -250) (`KismetMathLibrary.Conv_IntToDouble` (- (- (/ (+ (* (- (`self.Colomns`) 1) 50) (* (`self.Colomns`) 100)) 2) 50) (* (`local.I`) 150)))) (struct :`Yaw` -90.0)) "Undefined" "OverrideRootScale" null null))
  (return _returnvalue))

(fn `UserConstructionScript`)